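; Clock gate that the player opens by fading it out when holding the clock key.
; A Box overlap caches the ThirdPersonCharacter, creates the gate's dynamic material and enables input, which is disabled on exit.
; The clock_gate_open action checks HaskeyClock and either plays a locked sound or runs a timeline lowering the material's fade parameter.
; Each timeline update also replays the open sound and disables gate collision.
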(event OnComponentBeginOverlap(Box)
  (params (OverlappedComponent :type Primitive%20Component%20Object%20Reference) (OtherActor :type Actor%20Object%20Reference) (OtherComp :type Primitive%20Component%20Object%20Reference) (OtherBodyIndex :type Integer) (bFromSweep :type Boolean) (SweepResult :type Hit%20Result%20Structure%20%28by%20ref%29))
  (bind _asthird_person_character (Utilities|Casting|CastToThirdPersonCharacter OtherActor))
  (Input|EnableInput (Game|GetPlayerController 0))
  (bind _returnvalue (Rendering|Material|CreateDynamicMaterialInstance (Variables|Default|Getclock_gate) 0 "/Game/Narae/narae_material/clock_gate/clock_gate_material_2.clock_gate_material_2" "None" :!class /Script/Engine.PrimitiveComponent)))

(event OnComponentEndOverlap(Box)
  (params (OverlappedComponent :type Primitive%20Component%20Object%20Reference) (OtherActor :type Actor%20Object%20Reference) (OtherComp :type Primitive%20Component%20Object%20Reference) (OtherBodyIndex :type Integer))
  (Utilities|Casting|CastToThirdPersonCharacter OtherActor)
  (Input|DisableInput (Game|GetPlayerController 0)))

(event Input|ActionEvents|InputActionclock_gate_open
  (params (Key :type Key%20Structure :default "None"))
  (:Pressed
    (if (Variables|/Game/ThirdPersonBP/Blueprints/ThirdPersonCharacter.ThirdPersonCharacter_C|GetHaskey?_clock (stale OnComponentBeginOverlap(Box) _asthird_person_character))
      (bind _fade (Timeline|타임라인_0 Play)
        (:Update
          (Rendering|Material|SetScalarParameterValue (stale OnComponentBeginOverlap(Box) _returnvalue) "fade" (Math|Float|Lerp 1.0 0.0 _fade) :!class /Script/Engine.MaterialInstanceDynamic)
          (Audio|PlaySoundatLocation "/Game/Narae/narae_sound/clock_gate_open.clock_gate_open" (Transformation|GetActorLocation) "0, 0, 0" 1.0 1.0 0.0 0 0 0)
          (Collision|SetCollisionEnabled (Variables|Default|Getclock_gate) "NoCollision")
          (Variables|Default|SetbAutoDestroyWhenFinished true)))
      (else
        (Audio|PlaySoundatLocation "/Game/Narae/narae_sound/clock_gate_lock.clock_gate_lock" (Transformation|GetActorLocation) "0, 0, 0" 1.0 1.0 0.0 0 0 0)))))

(fn ConstructionScript)