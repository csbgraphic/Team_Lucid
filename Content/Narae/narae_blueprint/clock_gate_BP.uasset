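; Clock gate actor that the player raises or lowers with an input action, provided the character holds the clock key.
; A box overlap with the ThirdPersonCharacter enables input and opens a Gate node, and leaving reverses both.
; A FlipFlop alternates playing and reversing a timeline that lerps the gate's Z location, triggering the open sound on every update.
; Without the key, pressing plays a locked sound.
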(event OnComponentBeginOverlap(Box)
  (params (OverlappedComponent :type Primitive%20Component%20Object%20Reference) (OtherActor :type Actor%20Object%20Reference) (OtherComp :type Primitive%20Component%20Object%20Reference) (OtherBodyIndex :type Integer) (bFromSweep :type Boolean) (SweepResult :type Hit%20Result%20Structure%20%28by%20ref%29))
  (bind _asthird_person_character (Utilities|Casting|CastToThirdPersonCharacter OtherActor))
  (Input|EnableInput (Game|GetPlayerController 0))
  (Utilities|FlowControl|Gate true) ; enters at Open
)

(event OnComponentEndOverlap(Box)
  (params (OverlappedComponent :type Primitive%20Component%20Object%20Reference) (OtherActor :type Actor%20Object%20Reference) (OtherComp :type Primitive%20Component%20Object%20Reference) (OtherBodyIndex :type Integer))
  (Utilities|Casting|CastToThirdPersonCharacter OtherActor)
  (Input|DisableInput (Game|GetPlayerController 0))
  (Utilities|FlowControl|Gate true) ; enters at Close
)

(event Input|ActionEvents|InputActionclock_gate_open
  (params (Key :type Key%20Structure :default "None"))
  (:Pressed
    (if (Variables|/Game/ThirdPersonBP/Blueprints/ThirdPersonCharacter.ThirdPersonCharacter_C|GetHaskey?_clock (stale OnComponentBeginOverlap(Box) _asthird_person_character))
      (Utilities|FlowControl|Gate true
        (:Exit
          (Utilities|FlowControl|FlipFlop
            (:A
              (bind _open_gate (Timeline|open_gate Play)
                (:Update
                  (Transformation|SetRelativeLocation (Variables|Default|Getclock_gate) (Math|Vector|MakeVector 0.0 0.0 (Math|Float|Lerp (Variables|Default|Getclose) (Variables|Default|Getopen) _open_gate)) false false)
                  (Audio|PlaySoundatLocation "/Game/Narae/narae_sound/clock_gate_open.clock_gate_open" (Transformation|GetActorLocation) "0, 0, 0" 1.0 1.0 0.0 0 0 0))))
            (:B
              (Timeline|open_gate Reverse)))))
      (else
        (Audio|PlaySoundatLocation "/Game/Narae/narae_sound/clock_gate_lock.clock_gate_lock" (Transformation|GetActorLocation) "0, 0, 0" 1.0 1.0 0.0 0 0 0)))))

(fn ConstructionScript)